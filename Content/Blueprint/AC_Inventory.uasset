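; Inventory component that stores item stacks in a slot-keyed map and toggles the UMG_Inventory widget.
; PickUpItem tops up matching stacks up to each data asset's MaxStack, then uses the first empty slot unless the duplicate rule forbids it.
; Widget add and remove events write back to the map.
; Dropped items spawn as A_Item where a downward box trace ahead of the owner hits.
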(event `self.OpenInventory`
  (bind _returnvalue (`GameplayStatics.GetPlayerController` 0))
  (bind _as_umg_inven (`self.As UMG_Inven`))
  (`self.As UMG_Inven`
    (:`then`
      (`Widget.RemoveFromParent` (`self.As UMG_Inven`))
      (set `self.As UMG_Inven` null))
    (:`else`
      (bind _returnvalue_2 (`|CreateWidget` "/Game/UI/Hud/UMG_Inventory.UMG_Inventory_C" null (`self.Inventory`) (`self.MaxSize`) (`self.AllowDuplicate`)))
      (bind _output_get (set `self.As UMG_Inven` _returnvalue_2))
      (`UserWidget.AddToViewport` _output_get 0)
      (add `/Game/UI/Hud/UMG_Inventory.ItemAdded` _as_umg_inven (`|CreateDelegate` :!event `ItemAdded`))
      (add `/Game/UI/Hud/UMG_Inventory.ItemDropped` _as_umg_inven (`|CreateDelegate` :!event `ItemDropped`))
      (add `/Game/UI/Hud/UMG_Inventory.ItemRemoved` _as_umg_inven (`|CreateDelegate` :!event `ItemRemoved`))
      (set `PlayerController.bShowMouseCursor` true _returnvalue)
      (`WidgetBlueprintLibrary.SetInputMode_GameAndUIEx` _returnvalue null))))

(fn `IsKeyFull`
  (params (Key :type Integer))
  (returns (ReturnValue :type Boolean) (Remaining :type Integer))
  (bind (_value _returnvalue) (`BlueprintMapLibrary.Map_Find` (`self.Inventory`) (`local.Key`)))
  (bind (_quantity _dataasset) (break `/Game/Blueprint/ST_Inventory` _value))
  (bind _maxstack (`/Game/Blueprint/DA_Items.MaxStack` _dataasset))
  (bind _returnvalue_2 (- _maxstack _quantity))
  (if _returnvalue
    (return (and (== _returnvalue_2 0) (!= _maxstack 0)) _returnvalue_2)
    (else
      (return false -1))))

(fn `ItemAdded`
  (params (`Slot Key` :type Integer) (`Slot Value` :type "/Game/Blueprint/ST_Inventory Structure"))
  (`BlueprintMapLibrary.Map_Add` (`self.Inventory`) `Slot Key` `Slot Value`))

(fn `ItemDropped`
  (params (ItemDropped :type "/Game/Blueprint/ST_Inventory Structure"))
  (bind _returnvalue (`self.GetOwner`))
  (bind _returnvalue_2 (+ (* (`Actor.GetActorForwardVector` _returnvalue) 300) (`Actor.K2_GetActorLocation` _returnvalue)))
  (bind (_outhit _returnvalue_3) (`KismetSystemLibrary.BoxTraceSingle` _returnvalue_2 (- _returnvalue_2 (0.0 0.0 500.0)) (15.0 15.0 15.0) (struct) "TraceTypeQuery1" false (`|MakeArray` (`self.GetOwner`))))
  (if _returnvalue_3
    (`|SpawnActorFromClass` "/Game/Blueprint/A_Item.A_Item_C" (`KismetMathLibrary.MakeTransform` (`.ImpactPoint` (`GameplayStatics.BreakHitResult` _outhit))) "Undefined" "MultiplyWithRoot" null (`local.ItemDropped`) null)))

(fn `ItemRemoved`
  (params (Key :type Integer))
  (`BlueprintMapLibrary.Map_Remove` (`self.Inventory`) Key))

(fn `PickUpItem`
  (params (item :type "/Game/Blueprint/A_Item Object Reference"))
  (returns (ReturnValue :type Boolean))
  (locals (`L-QuantityIn` :type Integer) (`L-DataAssetIn` :type "/Game/Blueprint/DA_Items Object Reference") (`L-Index` :type Integer) (`L-FoundSameItem` :type Boolean) (`L-Remaining` :type Integer) (`L-EmptyKey` :type Integer :default -1))
  (bind (_quantity _dataasset) (break `/Game/Blueprint/ST_Inventory` (`/Game/Blueprint/A_Item.Structure` item)))
  (bind (_returnvalue _remaining) (`self.IsKeyFull` (`local.L-Index`)))
  (bind _value (`BlueprintMapLibrary.Map_Find` (`self.Inventory`) (`local.L-Index`)))
  (bind _returnvalue_2 (- (`local.L-QuantityIn`) (`local.L-Remaining`)))
  (set `local.L-QuantityIn` _quantity)
  (set `local.L-DataAssetIn` _dataasset)
  (while (and (> (`local.L-QuantityIn`) 0) (< (`local.L-Index`) (`self.MaxSize`)))
    (`|ExecutionSequence`
      (:`then_0`
        (if _returnvalue
          (if (== (`.DataAsset_5_8D7433EE4483A5B069608983E4BBF8DC` (break `/Game/Blueprint/ST_Inventory` (`BlueprintMapLibrary.Map_Find` (`self.Inventory`) (`local.L-Index`)))) (`local.L-DataAssetIn`))
            (set `local.L-FoundSameItem` true))
          (else
            (bind _output_get (set `local.L-Remaining` _remaining))
            (if (== _output_get -1)
              (if (== -1 (`local.L-EmptyKey`))
                (set `local.L-EmptyKey` (`local.L-Index`)))
              (elif (== (`.DataAsset_5_8D7433EE4483A5B069608983E4BBF8DC` (break `/Game/Blueprint/ST_Inventory` _value)) (`local.L-DataAssetIn`))
                (`BlueprintMapLibrary.Map_Add` (`self.Inventory`) (`local.L-Index`) (make `/Game/Blueprint/ST_Inventory` (+ (break `/Game/Blueprint/ST_Inventory` _value) (`KismetMathLibrary.Clamp` (`local.L-QuantityIn`) 0 (`local.L-Remaining`))) (`local.L-DataAssetIn`)))
                (set `local.L-QuantityIn` (`KismetMathLibrary.Clamp` _returnvalue_2 0 _returnvalue_2))
                (set `local.L-FoundSameItem` true))))))
      (:`then_1`
        (`/Engine/EditorBlueprintResources/StandardMacros.IncrementInt` (`local.L-Index`)))))
  (if (== (`local.L-QuantityIn`) 0)
    (return true)
    (elif (and (not (`self.AllowDuplicate`)) (`local.L-FoundSameItem`))
      (`/Game/Blueprint/A_Item.ModifyQuantity` (`local.item`) (`local.L-QuantityIn`))
      (return false)
      (elif (!= (`local.L-EmptyKey`) -1)
        (`BlueprintMapLibrary.Map_Add` (`self.Inventory`) (`local.L-EmptyKey`) (make `/Game/Blueprint/ST_Inventory` (`local.L-QuantityIn`) (`local.L-DataAssetIn`)))
        (return true)
        (else
          (return false))))))